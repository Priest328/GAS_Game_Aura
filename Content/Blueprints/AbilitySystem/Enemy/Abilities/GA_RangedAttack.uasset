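; GA_RangedAttack is an enemy gameplay ability that fires a projectile at the avatar's combat target.
; On activation it warps rotation toward the target and plays a random tagged attack montage.
; The montage's gameplay event triggers SpawnProjectile at its tagged socket, using the target's location re-read at that moment and an optional pitch override.
; The ability ends when the montage completes, is interrupted or cancelled, or when an interface cast fails.
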(event `self.K2_ActivateAbility`
  (bind _returnvalue (`self.GetAvatarActorFromActorInfo`))
  (bind _returnvalue_2 (`self.GetAvatarActorFromActorInfo`))
  (bind (_taggedmontage_montage _taggedmontage_montagetag _taggedmontage_sockettag) (break `TaggedMontage` (`self.TaggedMontage`)))
  (bind _taggedmontage_montage_2 (break `TaggedMontage` (`self.TaggedMontage`)))
  (cast `CombatInterface` _returnvalue
    (:`then`
      (cast `EnemyInterface` _returnvalue
        (:`then`
          (bind _returnvalue_3 (message `EnemyInterface.GetCombatTarget` _returnvalue_2))
          (message `CombatInterface.K2_WarpRotationToTarget` _returnvalue_2 (`Actor.K2_GetActorLocation` _returnvalue_3))
          (bind _returnvalue_4 (message `CombatInterface.GetAttackMontages` (`self.GetAvatarActorFromActorInfo`)))
          (set `self.TaggedMontage` (`self.GetRandomTaggedMontageFromArray` _returnvalue_4))
          (`AbilityTask_PlayMontageAndWait.CreatePlayMontageAndWaitProxy` "None" _taggedmontage_montage_2
            (:`then`
              (`AbilityTask_WaitGameplayEvent.WaitGameplayEvent` _taggedmontage_montagetag null true
                (:`EventReceived`
                  (bind _returnvalue_5 (message `EnemyInterface.GetCombatTarget` (`self.GetAvatarActorFromActorInfo`)))
                  (`self.SpawnProjectile` (`Actor.K2_GetActorLocation` _returnvalue_5) _taggedmontage_sockettag (`self.Should Override Pitch`) (`self.Pitch Override`)))))
            (:`OnCompleted`
              (`self.K2_EndAbility` :!label _label))
            (:`OnInterrupted`
              (goto _label))
            (:`OnCancelled`
              (goto _label))))
        (:`CastFailed`
          (`self.K2_EndAbility` :!label _label_2))))
    (:`CastFailed`
      (goto _label_2))))