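; Melee attack gameplay ability for enemies that deals damage to nearby hostile players during a randomly chosen attack montage.
; It motion-warps the avatar toward its combat target, plays the montage and waits for that montage's gameplay event.
; On the event, a small sphere query at the tagged combat socket damages non-friendly live players, and any hit fires a melee impact GameplayCue.
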(event `self.K2_ActivateAbility`
  (bind _returnvalue (`self.GetAvatarActorFromActorInfo`))
  (bind (_taggedmontage_montage _taggedmontage_montagetag) (break `TaggedMontage` (`self.TaggedMontage`)))
  (bind (_taggedmontage_montage_2 _taggedmontage_montagetag_2 _taggedmontage_sockettag) (break `TaggedMontage` (`self.TaggedMontage`)))
  (bind _taggedmontage_montage_3 (break `TaggedMontage` (`self.TaggedMontage`)))
  (set `self.HasHitTarget` false)
  (set `self.AvatarActor` _returnvalue)
  (cast `CombatInterface` _returnvalue)
  (bind _asenemy_interface (cast `EnemyInterface` _returnvalue))
  (message `CombatInterface.K2_WarpRotationToTarget` (`self.AvatarActor`) (`Actor.K2_GetActorLocation` (`EnemyInterface.GetCombatTarget` _asenemy_interface)))
  (bind _returnvalue_2 (message `CombatInterface.GetAttackMontages` (`self.AvatarActor`)))
  (set `self.TaggedMontage` (`self.GetRandomTaggedMontageFromArray` _returnvalue_2))
  (`AbilityTask_PlayMontageAndWait.CreatePlayMontageAndWaitProxy` "None" _taggedmontage_montage_3
    (:`then`
      (`AbilityTask_WaitGameplayEvent.WaitGameplayEvent` _taggedmontage_montagetag_2 null
        (:`EventReceived`
          (bind _returnvalue_3 (message `CombatInterface.GetCombatSocketLocation` (`self.AvatarActor`) _taggedmontage_sockettag))
          (set `self.CombatSocketLocation` _returnvalue_3)
          (bind _outoverlappingactors (`AuraAbilitySystemLibrary.GetLivePlayersWithinRadius` (`self.AvatarActor`) (`|MakeArray` (`self.AvatarActor`)) 75.0 (`self.CombatSocketLocation`)))
          (for _array_element _outoverlappingactors
            (if (`AuraAbilitySystemLibrary.IsNotFriend` (`self.AvatarActor`) _array_element)
              (`self.CauseDamage` _array_element)
              (set `self.HasHitTarget` true)))
          (if (`self.HasHitTarget`)
            (bind _returnvalue_4 (message `EnemyInterface.GetCombatTarget` (`self.AvatarActor`)))
            (`self.K2_ExecuteGameplayCueWithParams` (struct :`TagName` "GameplayCue.MeleeImpact") (`AbilitySystemBlueprintLibrary.MakeGameplayCueParameters` 0.0 0.0 (struct) (struct) (struct) (`BlueprintGameplayTagLibrary.MakeGameplayTagContainerFromTag` _taggedmontage_montagetag) (struct) (`self.CombatSocketLocation`) (0.0 0.0 0.0) null (`self.AvatarActor`) _returnvalue_4))
            (`self.K2_EndAbility`)
            (else
              (`self.K2_EndAbility`))))))
    (:`OnCompleted`
      (`self.K2_EndAbility` :!label _label))
    (:`OnInterrupted`
      (goto _label))
    (:`OnCancelled`
      (goto _label))))